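; Building_BP is a clickable building actor that opens its assigned mission on the player's pawn.
; Hovering the cursor over its Cube toggles custom depth rendering, and clicking it passes the Mission to Pawn_BP's CreateMissionWidget.
; The construction script writes BuildingName to a TextRender label, which turns every tick to face the pawn's camera.
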(event OnBeginCursorOver(Cube)
  (params (TouchedComponent :type Primitive%20Component%20Object%20Reference))
  (Rendering|SetRenderCustomDepth (Variables|Default|GetCube) true))

(event OnEndCursorOver(Cube)
  (params (TouchedComponent :type Primitive%20Component%20Object%20Reference))
  (Rendering|SetRenderCustomDepth (Variables|Default|GetCube) false))

(event OnClicked(Cube)
  (params (TouchedComponent :type Primitive%20Component%20Object%20Reference) (ButtonPressed :type Key%20Structure))
  (Default|CreateMissionWidget (Variables|Default|GetPawnRef) (Variables|Default|GetMission)))

(event EventBeginPlay
  (Variables|Default|SetPawnRef (.AsPawn%20BP (Utilities|Casting|CastToPawn_BP (Game|Player|GetPlayerPawn 0)))))

(event EventTick
  (params (DeltaSeconds :type Float%20%28single-precision%29))
  (bind _textrender (Variables|Default|GetTextRender))
  (Transformation|SetWorldRotation _textrender (Math|Rotator|FindLookatRotation (Transformation|GetWorldLocation _textrender) (Transformation|GetWorldLocation (Variables|/Game/Blueprints/Pawn_BP.Pawn_BP_C|GetCamera (Variables|Default|GetPawnRef)))) false false))

(fn ConstructionScript
  (Rendering|Components|TextRender|SetText (Variables|Default|GetTextRender) (Variables|Default|GetBuildingName)))