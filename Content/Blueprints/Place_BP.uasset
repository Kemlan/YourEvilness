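; Place actor that generates a random set of missions for itself on BeginPlay.
; Each mission is a spawned Mission_BP with a numbered description, filled with random counts of SkillTest_BP and Unit_BP actors.
; Skill tests get a random goal value and one of three tested skills.
; Both CreateMission and BeginPlay add the mission to the Mission array, so each is added twice.
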(event EventBeginPlay
  (for _index (range 0 (Math|Random|RandomIntegerinRange 1 3))
    (bind _missionref (CallFunction|CreateMission (Utilities|String|Append "Mission" (Utilities|String|ToString(Integer) (+ _index 1))) (Math|Random|RandomIntegerinRange 1 4) (Math|Random|RandomIntegerinRange 2 4)))
    (Utilities|Array|Add (Variables|Default|GetMission) _missionref)))

(fn ConstructionScript)

(fn CreateMission
  (params (Desc :type String) (NbSkillTest :type Integer) (NbUnit :type Integer))
  (bind _returnvalue (Game|SpawnActorfromClass "/Game/Blueprints/Mission_BP.Mission_BP_C" (Math|Conversions|ToTransform(Vector) "0, 0, 0") "Undefined" 0 Desc 0))
  (for _index (range 0 (- NbSkillTest 1))
    (CallFunction|CreateSkillTest _returnvalue))
  (for _index_2 (range 0 (- NbUnit 1))
    (CallFunction|CreateUnit _returnvalue))
  (Utilities|Array|Add (Variables|Default|GetMission) _returnvalue)
  (return _returnvalue))

(fn CreateUnit
  (params (Mission :type Mission%20BP%20Object%20Reference))
  (bind _returnvalue (Game|SpawnActorfromClass "/Game/Blueprints/Unit_BP.Unit_BP_C" (Transformation|GetActorTransform) "Undefined" 0 0 0))
  (Utilities|Array|Add (Variables|/Game/Blueprints/Mission_BP.Mission_BP_C|GetUnitList Mission) _returnvalue))

(fn CreateSkillTest
  (params (Mission :type Mission%20BP%20Object%20Reference))
  (bind _returnvalue (Game|SpawnActorfromClass "/Game/Blueprints/SkillTest_BP.SkillTest_BP_C" (Transformation|GetActorTransform) "Undefined" 0 0))
  (Variables|/Game/Blueprints/SkillTest_BP.SkillTest_BP_C|SetgoalValue _returnvalue (Math|Random|RandomIntegerinRange 1 9))
  (Variables|/Game/Blueprints/SkillTest_BP.SkillTest_BP_C|SetskillTested _returnvalue (Utilities|Select :Index (Math|Random|RandomIntegerinRange 0 2) :Option%200 "NewEnumerator0" :Option%201 "NewEnumerator1" :Option%202 "NewEnumerator2"))
  (Utilities|Array|Add (Variables|/Game/Blueprints/Mission_BP.Mission_BP_C|GetSkillTestList Mission) _returnvalue))