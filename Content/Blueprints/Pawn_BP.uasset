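; Player pawn that acts as a pannable, zoomable camera and manages the game's units, places and mission widget.
; BeginPlay spawns Unit_BP actors from ListUnit; helpers add randomized units or remove array entries, re-indexing each unit to match its slot.
; AddPlace spawns and tracks Place_BP actors at the pawn's transform, with itself as Instigator.
; Axis inputs drive movement and clamped spring-arm zoom, while events keep a single mission widget on screen.
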(event Custom|Create%20Mission%20Widget
  (params (WidgetClass :type User%20Widget%20Class%20Reference))
  (Utilities|IsValid (Variables|Default|GetmissionWidget)
    (:Is%20Not%20Valid
      (bind _returnvalue (UserInterface|CreateWidget WidgetClass))
      (bind _output_get (Variables|Default|SetmissionWidget _returnvalue))
      (UserInterface|Viewport|AddtoViewport _output_get 0))))

(event Custom|Remove%20Mission%20Widget
  (Widget|RemovefromParent (Variables|Default|GetmissionWidget))
  (Variables|Default|SetmissionWidget 0))

(event EventBeginPlay
  (for _index (range 0 (- (Utilities|Array|Length (Variables|Default|GetListUnit)) 1))
    (bind _returnvalue (Game|SpawnActorfromClass "/Game/Blueprints/Unit_BP.Unit_BP_C" (Math|Transform|MakeTransform "0, 0, 0") "Undefined" 0 (Utilities|String|EnumtoString (.Name (Utilities|Struct|BreakUnitInit_Struct (Utilities|Array|Get(acopy) (Variables|Default|GetListUnit) _index)))) (.Race (Utilities|Struct|BreakUnitInit_Struct (Utilities|Array|Get(acopy) (Variables|Default|GetListUnit) _index))) (.Might (Utilities|Struct|BreakUnitInit_Struct (Utilities|Array|Get(acopy) (Variables|Default|GetListUnit) _index))) (.Mind (Utilities|Struct|BreakUnitInit_Struct (Utilities|Array|Get(acopy) (Variables|Default|GetListUnit) _index))) (.Social (Utilities|Struct|BreakUnitInit_Struct (Utilities|Array|Get(acopy) (Variables|Default|GetListUnit) _index))) (.Magic (Utilities|Struct|BreakUnitInit_Struct (Utilities|Array|Get(acopy) (Variables|Default|GetListUnit) _index))) _index 0))
    (Utilities|Array|Add (Variables|Default|GetUnits) _returnvalue)))

(event Input|AxisEvents|InputAxisMoveForward
  (params (AxisValue :type Float%20%28single-precision%29))
  ;[1 1 1] Camera Move
  (Transformation|AddActorWorldOffset (Math|Vector|MakeVector (* AxisValue 3.0) 0.0 0.0)))

(event Input|AxisEvents|InputAxisMoveRight
  (params (AxisValue :type Float%20%28single-precision%29))
  ;[1 1 1] Camera Move
  (Transformation|AddActorWorldOffset (Math|Vector|MakeVector 0.0 (* AxisValue 3.0) 0.0)))

(event Input|AxisEvents|InputAxisZoomIn
  (params (AxisValue :type Float%20%28single-precision%29))
  (bind _springarm (Variables|Default|GetSpringArm))
  ;[1 1 1] Camera Move
  (Variables|/Script/Engine.SpringArmComponent|SetTargetArmLength _springarm (Math|Float|Clamp(Float) (- (Variables|/Script/Engine.SpringArmComponent|GetTargetArmLength _springarm) (* AxisValue 5.0)) 2e+02 4e+02)))

(fn ConstructionScript)

(fn AddPlace
  (params (Name :type String) (Description :type String) (initMission :type Array%20of%20Mission%20Init%20Struct%20Structures))
  (bind _returnvalue (Game|SpawnActorfromClass "/Game/Blueprints/Place_BP.Place_BP_C" (Transformation|GetActorTransform) "Undefined" 0 Name Description initMission self))
  (Utilities|Array|Add (Variables|Default|GetPlaces) _returnvalue)
  (return _returnvalue))

(fn GetUnit
  (params (index :type Integer))
  (return (Utilities|Array|Get(acopy) (Variables|Default|GetUnits) index)))

(fn AddRandomUnit
  (bind _returnvalue (Math|Random|RandomIntegerinRange 1 9))
  (bind _units (Variables|Default|GetUnits))
  (bind _returnvalue_2 (Game|SpawnActorfromClass "/Game/Blueprints/Unit_BP.Unit_BP_C" (Transformation|GetActorTransform self) "Undefined" 0 (Utilities|String|EnumtoString (Utilities|Enum|LiteralenumENames (Utilities|Enum|ByteToEnumENames (Math|Conversions|ToByte(Integer) (Math|Random|RandomIntegerinRange 1 9))))) "NewEnumerator0" _returnvalue _returnvalue _returnvalue _returnvalue (Utilities|Array|Length _units) 0))
  (Utilities|Array|Add _units _returnvalue_2))

(fn RemoveUnit
  (params (index :type Integer))
  (Utilities|Array|RemoveIndex (Variables|Default|GetUnits) index)
  (CallFunction|RefreshUnitIndex))

(fn RefreshUnitIndex
  (for _index (range 0 (- (Utilities|Array|Length (Variables|Default|GetUnits)) 1))
    (Variables|/Game/Blueprints/Unit_BP.Unit_BP_C|Setindex (Utilities|Array|Get(acopy) (Variables|Default|GetUnits) _index) _index)))